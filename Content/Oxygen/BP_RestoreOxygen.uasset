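; BP_RestoreOxygen is a plantable tree spot whose mesh the player changes with the 1, 2 or 3 key.
; Overlapping BoxOxygen enables input for player 0, and leaving disables it.
; Each key has a non-looping MultiGate stepping Planesadzonka through three meshes of one tree type, with its first press also enlarging BoxOxygen.
; No oxygen value is changed here, and the seedling mesh nodes are unconnected.
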(event `self.ReceiveActorBeginOverlap`
  (params (OtherActor :type "Actor Object Reference")))

(event `self.ReceiveTick`
  (params (DeltaSeconds :type "Float (single-precision)")))

(event `self.ReceiveBeginPlay`)

(event `self.BoxOxygen.OnComponentBeginOverlap`
  (params (OverlappedComponent :type "PrimitiveComponent Object Reference") (OtherActor :type "Actor Object Reference") (OtherComp :type "PrimitiveComponent Object Reference") (OtherBodyIndex :type Integer) (bFromSweep :type Boolean) (SweepResult :type "HitResult Structure (by ref)"))
  (`self.EnableInput` (`GameplayStatics.GetPlayerController` 0)))

(event `self.BoxOxygen.OnComponentEndOverlap`
  (params (OverlappedComponent :type "PrimitiveComponent Object Reference") (OtherActor :type "Actor Object Reference") (OtherComp :type "PrimitiveComponent Object Reference") (OtherBodyIndex :type Integer))
  (`self.DisableInput` (`GameplayStatics.GetPlayerController` 0)))

(event `Key|One`
  (params (Key :type "Key Structure"))
  (:`Pressed`
    (`|MultiGate` false
      (:`Out 0`
        (`StaticMeshComponent.SetStaticMesh` (`self.Planesadzonka`) "/Game/VRContent/Meshes/trees/tree1_1.tree1_1")
        (`SceneComponent.SetRelativeScale3D` (`self.BoxOxygen`) (10.0 10.0 10.0)))
      (:`Out 1`
        (`StaticMeshComponent.SetStaticMesh` (`self.Planesadzonka`) "/Game/VRContent/Meshes/trees/tree1_2.tree1_2"))
      (:`Out 2`
        (`StaticMeshComponent.SetStaticMesh` (`self.Planesadzonka`) "/Game/VRContent/Meshes/trees/tree1_3.tree1_3")))))

(event `Key|Two`
  (params (Key :type "Key Structure"))
  (:`Pressed`
    (`|MultiGate` false
      (:`Out 0`
        (`StaticMeshComponent.SetStaticMesh` (`self.Planesadzonka`) "/Game/VRContent/Meshes/trees/tree2_1.tree2_1")
        (`SceneComponent.SetRelativeScale3D` (`self.BoxOxygen`) (10.0 10.0 10.0)))
      (:`Out 1`
        (`StaticMeshComponent.SetStaticMesh` (`self.Planesadzonka`) "/Game/VRContent/Meshes/trees/tree2_2.tree2_2"))
      (:`Out 2`
        (`StaticMeshComponent.SetStaticMesh` (`self.Planesadzonka`) "/Game/VRContent/Meshes/trees/tree2_3.tree2_3")))))

(event `Key|Three`
  (params (Key :type "Key Structure"))
  (:`Pressed`
    (`|MultiGate` false
      (:`Out 0`
        (`StaticMeshComponent.SetStaticMesh` (`self.Planesadzonka`) "/Game/VRContent/Meshes/trees/tree3_3.tree3_3")
        (`SceneComponent.SetRelativeScale3D` (`self.BoxOxygen`) (10.0 10.0 10.0)))
      (:`Out 1`
        (`StaticMeshComponent.SetStaticMesh` (`self.Planesadzonka`) "/Game/VRContent/Meshes/trees/tree3_2.tree3_2"))
      (:`Out 2`
        (`StaticMeshComponent.SetStaticMesh` (`self.Planesadzonka`) "/Game/VRContent/Meshes/trees/tree3_1.tree3_1")))))

(fn `UserConstructionScript`)