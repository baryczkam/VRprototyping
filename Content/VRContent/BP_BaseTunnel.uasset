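; BP_BaseTunnel is a diggable block of dynamic mesh built with Geometry Script, which can be carved into tunnels at runtime.
; The construction script resets the mesh to a tessellated box and enables complex-as-simple collision.
; DigTunnel converts a given location into mesh space and boolean-subtracts a capsule there, using a temporary compute mesh that it releases afterwards.
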(fn `DigTunnel`
  (params (Location :type "Vector Structure"))
  (bind _returnvalue (`self.AllocateComputeMesh`))
  (bind _returnvalue_2 (`GeometryScriptLibrary_MeshPrimitiveFunctions.AppendCapsule` _returnvalue (struct) (`KismetMathLibrary.MakeTransform` (`KismetMathLibrary.InverseTransformLocation` (`SceneComponent.K2_GetComponentToWorld` (`self.DynamicMeshComponent`)) Location)) 30.0 75.0 5 12 "Center" null))
  (bind _returnvalue_3 (`BaseDynamicMeshComponent.GetDynamicMesh` (`self.DynamicMeshComponent`)))
  (`GeometryScriptLibrary_MeshBooleanFunctions.ApplyMeshBoolean` _returnvalue_3 (struct) _returnvalue_2 (struct) "Subtract" (struct) null)
  (`self.ReleaseAllComputeMeshes`))

(fn `UserConstructionScript`
  (bind _returnvalue (`BaseDynamicMeshComponent.GetDynamicMesh` (`self.DynamicMeshComponent`)))
  (bind _output_get (set `self.dynamicMesh` _returnvalue))
  (`DynamicMesh.Reset` _output_get)
  (bind _returnvalue_2 (`GeometryScriptLibrary_MeshPrimitiveFunctions.AppendBox` (`self.dynamicMesh`) (struct) (struct) 500.0 500.0 300.0 0 0 0 "Base" null))
  (`GeometryScriptLibrary_MeshSubdivideFunctions.ApplyPNTessellation` _returnvalue_2 (struct) 2 null)
  (`DynamicMeshComponent.SetComplexAsSimpleCollisionEnabled` (`self.DynamicMeshComponent`) true true))